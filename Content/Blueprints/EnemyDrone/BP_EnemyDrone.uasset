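; Enemy drone that chases a target pawn, fires blasters at it and explodes when its health runs out.
; BeginPlay stores the first Pawn found as the target, and Tick smoothly turns toward it while moving forward without sweep.
; A looping timer alternates left and right rifle sockets via FlipFlop, spawning aimed beams with burst effects and a sound played at world origin.
; GetHurt subtracts damage and handles destruction.
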(event `self.ReceiveBeginPlay`
  (`self.StoreTargetPawn`)
  (`KismetSystemLibrary.K2_SetTimerDelegate` (delegate `FireBlasterEvent`) (`self.BlasterTime`) true))

(event `FireBlasterEvent`
  (`/Engine/EditorBlueprintResources/StandardMacros.FlipFlop`
    (:`A`
      (`self.SpawnBlasterBeam` "Rifle_L"))
    (:`B`
      (`self.SpawnBlasterBeam` "Rifle_R"))))

(event `self.ReceiveTick`
  (params (DeltaSeconds :type "Float (single-precision)"))
  ;[0 0.0436 0.15 0.5] Interpolate Rotation to TargetPawn
  (`self.InterpRotation` DeltaSeconds (`self.rotationInterpSpeed`))
  (`self.MoveDroneForward`))

(event `/Game/Blueprints/Interfaces/BPI_Damagable.GetHurt`
  (params (Damage :type "Float (double-precision)"))
  (bind _returnvalue (`self.K2_GetActorLocation`))
  (bind _output_get (set `self.Health` (- (`self.Health`) Damage)))
  (if (<= _output_get 0.0)
    (`NiagaraFunctionLibrary.SpawnSystemAtLocation` "/Game/Global/Effects/Projectiles/FireExplosion/NS_FireExplosion.NS_FireExplosion" _returnvalue)
    (`GameplayStatics.PlaySoundAtLocation` "/Game/Global/Sounds/Explode/sfx_FireBolt_Impact.sfx_FireBolt_Impact" _returnvalue (struct) 1.0 1.0 0.0 null null null null)
    (`self.K2_DestroyActor`)))

(fn `FindTargetRotation`
  (returns (TargetRotation :type "Rotator Structure"))
  (return (`KismetMathLibrary.FindLookAtRotation` (`self.K2_GetActorLocation`) (`self.K2_GetActorLocation` (`self.Player`)))))

(fn `InterpRotation`
  (params (DeltaTime :type "Float (single-precision)") (InterpSpeed :type "Float (single-precision)"))
  (`self.Player`
    (:`then`
      (`self.K2_SetActorRotation` (`KismetMathLibrary.RInterpTo` (`self.K2_GetActorRotation`) (`self.FindTargetRotation`) DeltaTime InterpSpeed)))
    (:`else`)))

(fn `MoveDroneForward`
  (`self.K2_AddActorWorldOffset` (* (* (`self.Speed`) (`GameplayStatics.GetWorldDeltaSeconds`)) (`self.GetActorForwardVector`))))

(fn `SpawnBlasterBeam`
  (params (SocketName :type Name))
  (bind _drone (`self.Drone`))
  (bind _returnvalue_location (`KismetMathLibrary.BreakTransform` (`SceneComponent.GetSocketTransform` _drone SocketName "RTS_World")))
  (`|SpawnActorFromClass` (`self.BlasterBeamClass`) (`KismetMathLibrary.MakeTransform` _returnvalue_location (`KismetMathLibrary.FindLookAtRotation` _returnvalue_location (`self.K2_GetActorLocation` (`self.Player`))) (`self.GetActorScale3D`)) "Undefined" "MultiplyWithRoot" null null)
  (`NiagaraFunctionLibrary.SpawnSystemAtLocation` "/Game/Assets/FX/NS_BeamBurst.NS_BeamBurst" (`SceneComponent.GetSocketLocation` _drone SocketName))
  (`GameplayStatics.PlaySoundAtLocation` "/Game/Assets/Sounds/Drone/SFX_EnergyRifle.SFX_EnergyRifle" (0.0 0.0 0.0) (struct) 1.0 1.0 0.0 null null null null))

(fn `StoreTargetPawn`
  (bind _outactors (`GameplayStatics.GetAllActorsOfClass` "/Script/Engine.Pawn"))
  (if (`KismetArrayLibrary.Array_IsValidIndex` _outactors)
    (set `self.Player` (`|GetArrayItem` _outactors))))

(fn `UserConstructionScript`)