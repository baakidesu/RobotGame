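; BP_BotSpawner is a one-shot trigger volume that spawns enemy drones when something begins overlapping its box.
; The first overlap sets a DidSpawn guard, then spawns a BP_EnemyDrone at the location of each valid actor in the TargetPoints array.
; The spawner destroys itself afterward, and debug prints report overlaps and invalid target points.
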(event `self.Box.OnComponentBeginOverlap`
  (params (OverlappedComponent :type "PrimitiveComponent Object Reference") (OtherActor :type "Actor Object Reference") (OtherComp :type "PrimitiveComponent Object Reference") (OtherBodyIndex :type Integer) (bFromSweep :type Boolean) (SweepResult :type "HitResult Structure (by ref)"))
  (`KismetSystemLibrary.PrintString` "Hello")
  (if (not (`self.didSpawn`))
    (set `self.didSpawn` true)
    (for _array_element (`self.TargetPoints`)
      (`/Engine/EditorBlueprintResources/StandardMacros.IsValid` _array_element
        (:`Is Valid`
          (`|SpawnActorFromClass` "/Game/Blueprints/EnemyDrone/BP_EnemyDrone.BP_EnemyDrone_C" (`KismetMathLibrary.MakeTransform` (`self.K2_GetActorLocation` _array_element)) "Undefined" "MultiplyWithRoot" null null))
        (:`Is Not Valid`
          (`KismetSystemLibrary.PrintString` "not valid"))))
    (`self.K2_DestroyActor`)))

(fn `UserConstructionScript`)