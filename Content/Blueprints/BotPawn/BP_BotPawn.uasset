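; Player-controlled flying drone pawn that adds the HUD and Enhanced Input context on BeginPlay and turns its mesh to match control rotation each tick.
; Move input drives FloatingPawnMovement along control-rotation axes, and look input adds yaw and pitch.
; Firing alternates left and right rifle sockets, aiming each spawned beam at a camera line-trace hit or range end, with burst effect and sound.
; GetHurt subtracts health and quits the game at zero.
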(event `self.ReceiveTick`
  (params (DeltaSeconds :type "Float (single-precision)"))
  (`SceneComponent.K2_SetWorldRotation` (`self.DroneMesh`) (`self.GetControlRotation`) false false))

(event `self.ReceiveBeginPlay`
  ;[0.1272 0 0.15 0.5] Add OverlayHUD to viewport
  (bind _returnvalue (`|CreateWidget` "/Game/Blueprints/UI/WBP_OverlayHUD.WBP_OverlayHUD_C"))
  (`UserWidget.AddToViewport` _returnvalue 0)
  ;[0 0.0503 0.15 0.5] Add Drone Input Mapping Context
  (bind _asplayer_controller (cast `PlayerController` (`self.GetController`)))
  (bind _output_get (set `self.PlayerController` _asplayer_controller))
  (`EnhancedInputSubsystemInterface.AddMappingContext` (pcsubsystem `EnhancedInputLocalPlayerSubsystem` _output_get) "/Game/Blueprints/Input/IMC_Drone.IMC_Drone" 0 (struct)))

(event `EnhancedInput|/Game/Blueprints/Input/IA_Fire`
  (params (ActionValue :type Boolean) (ElapsedSeconds :type "Float (double-precision)") (TriggeredSeconds :type "Float (double-precision)") (InputAction :type "InputAction Object Reference" :default "/Game/Blueprints/Input/IA_Fire.IA_Fire"))
  ;[0.1272 0 0.15 0.5] Shoot
  (:`Triggered`
    (bind _isa (`/Engine/EditorBlueprintResources/StandardMacros.FlipFlop`)
      (:`A`
        _)
      (:`B`
        _))
    (`self.SpawnBlasterBeam` _isa)))

(event `EnhancedInput|/Game/Blueprints/Input/IA_Look`
  (params (ActionValue :type "Vector2D Structure") (ElapsedSeconds :type "Float (double-precision)") (TriggeredSeconds :type "Float (double-precision)") (InputAction :type "InputAction Object Reference" :default "/Game/Blueprints/Input/IA_Look.IA_Look"))
  (:`Triggered`
    (`self.AddControllerYawInput` ActionValue_X)
    (`self.AddControllerPitchInput` ActionValue_Y)))

(event `EnhancedInput|/Game/Blueprints/Input/IA_Move`
  (params (ActionValue :type "Vector Structure") (ElapsedSeconds :type "Float (double-precision)") (TriggeredSeconds :type "Float (double-precision)") (InputAction :type "InputAction Object Reference" :default "/Game/Blueprints/Input/IA_Move.IA_Move"))
  (:`Triggered`
    (`PawnMovementComponent.AddInputVector` (`self.FloatingPawnMovement`) (* ActionValue_X (`KismetMathLibrary.GetRightVector` (`self.GetControlRotation`))) false)
    (`PawnMovementComponent.AddInputVector` (`self.FloatingPawnMovement`) (* (`KismetMathLibrary.GetForwardVector` (`self.GetControlRotation`)) ActionValue_Y) false)
    (`PawnMovementComponent.AddInputVector` (`self.FloatingPawnMovement`) (* (`KismetMathLibrary.GetUpVector` (`self.GetControlRotation`)) ActionValue_Z) false)))

(event `/Game/Blueprints/Interfaces/BPI_Damagable.GetHurt`
  (params (Damage :type "Float (double-precision)"))
  (bind _output_get (set `self.Health` (- (`self.Health`) Damage)))
  (`KismetSystemLibrary.PrintString` (`KismetStringLibrary.Concat_StrStr` "Took damage! Health: " (`KismetStringLibrary.Conv_DoubleToString` _output_get)))
  (if (<= (`self.Health`) 0.0)
    (`KismetSystemLibrary.QuitGame` null "Quit")))

(fn `SpawnBlasterBeam`
  (params (`Is Left` :type Boolean))
  (bind _returnvalue_location (`KismetMathLibrary.BreakTransform` (`SceneComponent.GetSocketTransform` (`self.DroneMesh`) (`self.SocketName`) "RTS_World")))
  (`self.SetTraceStartAndEnd`
    (:`Output`
      (bind _outhit (`KismetSystemLibrary.LineTraceSingle` :`Start` (`self.TraceStart`) :`End` (`self.TraceEnd`) :`TraceChannel` "TraceTypeQuery1" :`DrawDebugType` "ForDuration"))
      (bind (_bblockinghit _binitialoverlap _time _distance _location _impactpoint) (`GameplayStatics.BreakHitResult` _outhit))
      (set `self.TraceEnd` (`KismetMathLibrary.SelectVector` _impactpoint (`self.TraceEnd`) _bblockinghit))
      (if (`local.Is Left`)
        (set `self.SocketName` "Rifle_L")
        (else
          (set `self.SocketName` "Rifle_R")))
      (`|SpawnActorFromClass` "/Game/Blueprints/BlasterBeam/BP_PlayerBlasterBeam.BP_PlayerBlasterBeam_C" (`KismetMathLibrary.MakeTransform` _returnvalue_location (`KismetMathLibrary.FindLookAtRotation` _returnvalue_location (`self.TraceEnd`))) "Undefined" "MultiplyWithRoot" null null null)
      (`NiagaraFunctionLibrary.SpawnSystemAtLocation` "/Game/Assets/FX/NS_BeamBurst.NS_BeamBurst" (`SceneComponent.GetSocketLocation` (`self.DroneMesh`) (`self.SocketName`)))
      (`GameplayStatics.PlaySoundAtLocation` "/Game/Assets/Sounds/Drone/SFX_EnergyRifle.SFX_EnergyRifle" (0.0 0.0 0.0) (struct) 1.0 1.0 0.0 null null null null))))

(fn `UserConstructionScript`)