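; BP_SmallSphere is a short-lived, moving, spinning pickup sphere that increments the score when a Pawn overlaps it.
; Tick moves it along its forward vector and applies a random spin set at BeginPlay, so the rotation also steers its path.
; Timelines scale it in on spawn and out on pickup or lifetime expiry, with a guard against repeat wink-outs, then destroy it.
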(event `self.ReceiveBeginPlay`
  (`self.WinkIn`)
  (`self.InitializeDeltaRotation`)
  ;[0.1272 0 0.15 0.5] Start WinkOut Timeline
  (`KismetSystemLibrary.K2_SetTimerDelegate` (delegate `WinkOut`) (`self.Lifetime`))
  ;[0.1272 0 0.15 0.5] Handle Overlap
  (add `PrimitiveComponent.OnComponentBeginOverlap` (`self.SphereVolume`) (delegate `OnSphereOverlap`)))

(event `OnSphereOverlap`
  (params (OverlappedComponent :type "PrimitiveComponent Object Reference") (OtherActor :type "Actor Object Reference") (OtherComp :type "PrimitiveComponent Object Reference") (OtherBodyIndex :type Integer) (bFromSweep :type Boolean) (SweepResult :type "HitResult Structure (by ref)"))
  ;[0.1272 0 0.15 0.5] Handle Overlap
  (if (`GameplayStatics.ObjectIsA` OtherActor "/Script/Engine.Pawn")
    (bind _asbp_robot_project_game_mode (cast `/Game/Blueprints/Game/BP_RobotProjectGameMode` (`GameplayStatics.GetGameMode`)))
    (`/Game/Blueprints/Game/BP_RobotProjectGameMode.IncrementScore` _asbp_robot_project_game_mode)
    (`self.WinkOut`)))

(event `WinkOut`
  ;[0.1272 0 0.15 0.5] Start WinkOut Timeline
  (if (not (`self.IsWinking`))
    (set `self.IsWinking` true)
    (bind (_direction _scale) (`Timeline|WinkOutTimeline`)
      (:`Update`
        (`SceneComponent.SetWorldScale3D` (`self.SmallSphere`) (`KismetMathLibrary.MakeVector` _scale _scale _scale)))
      (:`Finished`
        (`self.K2_DestroyActor`)))))

(event `self.ReceiveTick`
  (params (DeltaSeconds :type "Float (single-precision)"))
  ;[0.1272 0 0.15 0.5] Update Rot and Loc
  (`self.Move` DeltaSeconds)
  (`self.UpdateRotation` DeltaSeconds))

(event `WinkIn`
  ;[0.1272 0 0.15 0.5] Wink Into Existance
  (bind (_direction _scale) (`Timeline|Wink In`)
    (:`Update`
      (`SceneComponent.SetWorldScale3D` (`self.SmallSphere`) _scale))))

(event `self.SphereVolume.OnComponentBeginOverlap`
  (params (OverlappedComponent :type "PrimitiveComponent Object Reference") (OtherActor :type "Actor Object Reference") (OtherComp :type "PrimitiveComponent Object Reference") (OtherBodyIndex :type Integer) (bFromSweep :type Boolean) (SweepResult :type "HitResult Structure (by ref)")))

(fn `InitializeDeltaRotation`
  (set `self.DeltaRot` (* (`KismetMathLibrary.RandomRotator` false) (`self.RotationScaleFactor`))))

(fn `Move`
  (params (DeltaSeconds :type "Float (double-precision)"))
  (`self.K2_AddActorWorldOffset` (* (* DeltaSeconds (`self.MoveSpeed`)) (`self.GetActorForwardVector`))))

(fn `UpdateRotation`
  (params (DeltaSeconds :type "Float (double-precision)"))
  (`self.K2_AddActorWorldRotation` (* (`self.DeltaRot`) DeltaSeconds)))

(fn `UserConstructionScript`)